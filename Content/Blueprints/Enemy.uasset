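; Enemy actor that, once in camera view, drifts along -Y, fires projectiles and dodges vertically at random.
; Tick drives movement input unless Dashing, while a random Delay on the same Tick paces EnemyProjectile spawns from Arrow1 and occasional brief up or down jinks.
; Hits reduce health; death switches capsule and hitbox collision type and steers the enemy downward until Deathcollision destroys it.
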(event Custom|Death
  ;[1 1 1] Death
  (Variables|Default|SetIsdead true)
  (Collision|SetCollisionObjectType (Variables|Collision|GetCapsuleComponent) "ECC_GameTraceChannel9"))

(event EventDeathcollision
  ;[1 1 1] Death
  (Actor|DestroyActor))

(event EventTick
  (params (DeltaSeconds :type Float%20%28single-precision%29))
  ;[1 1 1] Behavior
  (if (Variables|Default|GetIsdead)
    (Pawn|Input|AddMovementInput "0,-0.500000,-2.000000" 0.5 false)
    (else
      (Utilities|FlowControl|Sequence
        (:then_0
          (if (Variables|Default|GetIncamera)
            (Utilities|FlowControl|Delay (Math|Random|RandomFloatinRange 0.5 2.0))
            (Game|SpawnActorfromClass "/Game/Blueprints/EnemyProjectile.EnemyProjectile_C" (Transformation|GetWorldTransform (Variables|Default|GetArrow1)) "Undefined" 0 0)
            (if (Math|Random|RandomBoolwithWeight 0.3)
              (if (Math|Random|RandomBoolwithWeight 0.5)
                (Variables|Default|SetMovement "0, 0,1.400000")
                (Utilities|FlowControl|Delay 0.1)
                (else
                  (Variables|Default|SetMovement "0, 0,-1.400000")
                  (Utilities|FlowControl|Delay 0.1)))
              (Variables|Default|SetMovement "0,-0.300000,0.000000"))))
        (:then_1
          (if (not (Variables|Default|GetDashing))
            (Pawn|Input|AddMovementInput (Variables|Default|GetMovement) 0.5 false)))))))

(event EventHitbyPlayer
  (params (Damage :type Float%20%28single-precision%29))
  ;[1 1 1] Getdamage
  (Variables|Default|SetHealthpoints (- (Variables|Default|GetHealthpoints) Damage))
  (if (< (Variables|Default|GetHealthpoints) 1.0)
    (CallFunction|Death)))

(event EventEntertheCamera
  ;[1 1 1] Behavior
  (Variables|Default|SetMovement "0,-0.300000, 0")
  (Variables|Default|SetIncamera true))

(fn ConstructionScript)