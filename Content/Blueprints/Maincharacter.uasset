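; Player character for a 2D flipbook shooter, moving on the Y/Z plane and creating the main UI on BeginPlay.
; Hits reduce HP, granting brief invulnerability with a damage flipbook, or destroy the actor at depletion.
; Dash spends regenerating boost to temporarily swap collision channel and raise fly speed and acceleration during a timeline.
; Held fire loops through a gate and retriggerable delay, spawning projectiles from limited ammo with timed reloads.
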(event Custom|Receive%20Damage
  (params (NewParam :type Float%20%28single-precision%29))
  ;[1 1 1] Damage/Death
  (Variables|Default|SetCurrentHP (- (Variables|Default|GetCurrentHP) NewParam))
  (if (< (Variables|Default|GetCurrentHP) 1.0)
    (Actor|DestroyActor)
    (else
      (Variables|Default|SetGotdamage true)
      (Sprite|SetFlipbook (Variables|Default|GetPaperFlipbook) "/Game/Assets/Sprites/Characters/Main/PlayerDamage.PlayerDamage")
      (Utilities|FlowControl|Delay 1.5)
      (Variables|Default|SetGotdamage false)
      (Sprite|SetFlipbook (Variables|Default|GetPaperFlipbook) "/Game/Assets/Sprites/Characters/Main/PlayerIdle.PlayerIdle"))))

(event EventBeginPlay
  ;[1 1 1] Cast UI
  (bind _returnvalue (UserInterface|CreateWidget "/Game/Blueprints/MainUI.MainUI_C"))
  (bind _output_get (Variables|Default|SetHP%20Reference _returnvalue))
  (UserInterface|Viewport|AddtoViewport _output_get 0))

(event EventTick
  (params (DeltaSeconds :type Float%20%28single-precision%29))
  ;[1 1 1] Dash
  (Utilities|FlowControl|Delay 0.5)
  (if (not (== (Variables|Default|GetCurrentBoost) (Variables|Default|GetMaxBoost)))
    (Variables|Default|SetCurrentBoost (+ (Variables|Default|GetCurrentBoost) 2.0))))

(event EventEnemyHit
  (params (Damage%20amount :type Float%20%28single-precision%29))
  ;[1 1 1] Damage/Death
  (if (Variables|Default|GetGotdamage)
    (Development|PrintString "nodamagenow")
    (else
      (CallFunction|ReceiveDamage Damage%20amount))))

(event Input|ActionEvents|InputActionShoot
  (params (Key :type Key%20Structure :default "None"))
  ;[1 1 1] Shoot and Reload
  (:Pressed
    (Utilities|FlowControl|Sequence
      (:then_0
        (goto _label Open))
      (:then_1
        (Utilities|FlowControl|Gate true :!label _label
          (:Exit
            (Utilities|FlowControl|Sequence
              (:then_0
                (if (not (Variables|Default|GetReloading))
                  (if (> (Variables|Default|Getammo) 0.0)
                    (Game|SpawnActorfromClass "/Game/Blueprints/Playerprojectile.Playerprojectile_C" (Transformation|GetWorldTransform (Variables|Default|GetGun)) "Undefined" 0 0)
                    (bind _result (Math|Float|DecrementFloat (Variables|Default|Getammo))
                      (:%20%20
                        (Development|PrintString (Utilities|String|ToString(Float) _result))))
                    (else
                      (Development|PrintString "out of ammo")))))
              (:then_1
                (Utilities|FlowControl|RetriggerableDelay (Variables|Default|GetShootInterval))
                (goto _label))))))))
  (:Released
    (goto _label Close)))

(event Input|ActionEvents|InputActionReload
  (params (Key :type Key%20Structure :default "None"))
  ;[1 1 1] Shoot and Reload
  (:Pressed
    (Development|PrintString "Is reloading")
    (Variables|Default|SetReloading true)
    (Utilities|FlowControl|Delay 1.2)
    (Variables|Default|Setammo 25.0)
    (Variables|Default|SetReloading false)))

(event Input|ActionEvents|InputActionDash
  (params (Key :type Key%20Structure :default "None"))
  (bind _charactermovement (Variables|Character|GetCharacterMovement))
  (bind _charactermovement_2 (Variables|Character|GetCharacterMovement))
  ;[1 1 1] Dash
  (:Pressed
    (if (not (< (Variables|Default|GetCurrentBoost) 2e+01))
      (Variables|Default|SetCurrentBoost (- (Variables|Default|GetCurrentBoost) 2e+01))
      (Collision|SetCollisionObjectType (Variables|Collision|GetCapsuleComponent) "ECC_GameTraceChannel4")
      (Sprite|SetFlipbook (Variables|Default|GetPaperFlipbook) "/Game/Assets/Sprites/Characters/Main/PlayerDash.PlayerDash")
      (Variables|/Script/Engine.CharacterMovementComponent|SetMaxAcceleration _charactermovement_2 2e+04)
      (Variables|/Script/Engine.CharacterMovementComponent|SetMaxFlySpeed _charactermovement_2 2e+03)
      (Timeline|Dash PlayFromStart
        (:Update
          (Pawn|Input|AddMovementInput "0, 0, 0" 1.0 false))
        (:Finished
          (Collision|SetCollisionObjectType (Variables|Collision|GetCapsuleComponent) "ECC_GameTraceChannel2")
          (Variables|/Script/Engine.CharacterMovementComponent|SetMaxAcceleration _charactermovement 4e+03)
          (Variables|/Script/Engine.CharacterMovementComponent|SetMaxFlySpeed _charactermovement 4.5e+02)
          (Sprite|SetFlipbook (Variables|Default|GetPaperFlipbook) "/Game/Assets/Sprites/Characters/Main/PlayerIdle.PlayerIdle"))))))

(event Input|AxisEvents|InputAxisMoveUp/Down
  (params (AxisValue :type Float%20%28single-precision%29))
  ;[1 1 1] Movement
  (Pawn|Input|AddMovementInput "0.000000,0.000000,1.000000" AxisValue false))

(event Input|AxisEvents|InputAxisMoveLeftRight
  (params (AxisValue :type Float%20%28single-precision%29))
  ;[1 1 1] Movement
  (Pawn|Input|AddMovementInput "0.000000,1.000000, 0" AxisValue false))

(fn ConstructionScript)