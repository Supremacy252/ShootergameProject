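; Flipbook-based enemy bomb projectile that detonates on touching the main character, after a short fuse, or when player hits deplete its HP.
; The fuse swaps flipbook states, then detonation disables the capsule, changes the blast radius's collision channel and plays a timeline that scales the explosion sprite.
; Blast-radius overlaps send damage through the HitbyEnemy interface.
; The bomb destroys itself after a brief delay, or immediately on Deathcollision.
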(event OnComponentBeginOverlap(Bombradius)
  (params (OverlappedComponent :type Primitive%20Component%20Object%20Reference) (OtherActor :type Actor%20Object%20Reference) (OtherComp :type Primitive%20Component%20Object%20Reference) (OtherBodyIndex :type Integer) (bFromSweep :type Boolean) (SweepResult :type Hit%20Result%20Structure%20%28by%20ref%29))
  (if (Utilities|DoesObjectImplementInterface OtherActor "/Game/Blueprints/InteractionBlueprints/HitbyEnemy.HitbyEnemy_C")
    (Class|HitbyEnemy|EnemyHit(Message) OtherActor (Variables|Default|GetDamageamount))))

(event Custom|Bombtrigger
  (Collision|SetCollisionEnabled (Variables|Default|GetCapsule) "NoCollision")
  (Collision|SetCollisionObjectType (Variables|Default|GetBombradius) "ECC_GameTraceChannel6")
  (Sprite|SetFlipbook (Variables|Default|GetBombS) "/Game/Assets/Sprites/Projectiles/Bomb/BombState3.BombState3")
  (bind _increasment (Timeline|Explosion Play)
    (:Update
      (Transformation|SetWorldTransform (Variables|Default|GetBombS) (Math|Transform|MakeTransform (Transformation|GetWorldLocation (Variables|Default|GetBombS)) "0,-90.000000, 0" (Math|Conversions|ToVector(Float) _increasment)) false false)
      (Utilities|FlowControl|Delay 0.4)
      (Actor|DestroyActor))))

(event EventDeathcollision
  (Actor|DestroyActor))

(event EventBeginPlay
  (Utilities|FlowControl|Delay 1.0)
  (if (not (Variables|Default|GetDestroyed))
    (Sprite|SetFlipbook (Variables|Default|GetBombS) "/Game/Assets/Sprites/Projectiles/Bomb/BombState2.BombState2")
    (Utilities|FlowControl|Delay 0.5)
    (if (not (Variables|Default|GetDestroyed))
      (CallFunction|Bombtrigger))))

(event EventHitbyPlayer
  (params (Damage :type Float%20%28double-precision%29))
  (Variables|Default|SetHP (- (Variables|Default|GetHP) Damage))
  (Audio|PlaySoundatLocation "/Game/FX/SFX/EnemygotHit.EnemygotHit" "0, 0, 0" "0, 0, 0" 1.0 1.0 0.0 0 0 0 0)
  (if (< (Variables|Default|GetHP) 1.0)
    (Variables|Default|SetDestroyed true)
    (CallFunction|Bombtrigger)))

(event Collision|EventActorBeginOverlap
  (params (OtherActor :type Actor%20Object%20Reference))
  (Utilities|Casting|CastToMaincharacter OtherActor)
  (Collision|SetCollisionEnabled (Variables|Default|GetCapsule) "NoCollision")
  (Collision|SetCollisionObjectType (Variables|Default|GetBombradius) "ECC_GameTraceChannel6")
  (Sprite|SetFlipbook (Variables|Default|GetBombS) "/Game/Assets/Sprites/Projectiles/Bomb/BombState3.BombState3")
  (bind _increasment (Timeline|Explosion Play)
    (:Update
      (Transformation|SetWorldTransform (Variables|Default|GetBombS) (Math|Transform|MakeTransform (Transformation|GetWorldLocation (Variables|Default|GetBombS)) "0,-90.000000, 0" (Math|Conversions|ToVector(Float) _increasment)) false false)
      (Utilities|FlowControl|Delay 0.4)
      (Actor|DestroyActor))))

(fn ConstructionScript)