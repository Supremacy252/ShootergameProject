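; Bomber enemy that starts its movement when it enters the camera, takes player hits and damages overlapped actors through the HitbyEnemy interface.
; Tick drives movement and a random Delay that repeatedly spawns Bombs at Arrow1, but only while Soundenabled is set.
; At zero health it switches collision channel and sinks diagonally until Deathcollision destroys it.
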(event OnComponentBeginOverlap(CapsuleComponent)
  (params (OverlappedComponent :type Primitive%20Component%20Object%20Reference) (OtherActor :type Actor%20Object%20Reference) (OtherComp :type Primitive%20Component%20Object%20Reference) (OtherBodyIndex :type Integer) (bFromSweep :type Boolean) (SweepResult :type Hit%20Result%20Structure%20%28by%20ref%29))
  ;[1 1 1] CollisionDamage
  (if (Utilities|DoesObjectImplementInterface OtherActor "/Game/Blueprints/InteractionBlueprints/HitbyEnemy.HitbyEnemy_C")
    (Class|HitbyEnemy|EnemyHit(Message) OtherActor (Variables|Default|GetCOllisiondamage))))

(event Custom|Death
  ;[1 1 1] Death
  (Variables|Default|SetIsdead true)
  (Collision|SetCollisionObjectType (Variables|Collision|GetCapsuleComponent) "ECC_GameTraceChannel9"))

(event EventDeathcollision
  ;[1 1 1] Death
  (Actor|DestroyActor))

(event EventSoundon
  ;[1 1 1] Behavior
  (Variables|Default|SetSoundenabled true))

(event EventSoundoff
  ;[1 1 1] Behavior
  (Variables|Default|SetSoundenabled false))

(event EventTick
  (params (DeltaSeconds :type Float%20%28single-precision%29))
  ;[1 1 1] Behavior
  (if (Variables|Default|GetIsdead)
    (Pawn|Input|AddMovementInput "0,-0.500000,-2.000000" 0.5 false)
    (else
      (Utilities|FlowControl|Sequence
        (:then_0
          (if (Variables|Default|GetSoundenabled)
            (Utilities|FlowControl|Delay (Math|Random|RandomFloatinRange 1.0 2.0))
            (if (Variables|Default|GetSoundenabled)
              (Audio|PlaySoundatLocation (Variables|Default|GetShootsound) "0, 0, 0" "0, 0, 0" 1.0 1.0 0.0 0 0 0))
            (Game|SpawnActorfromClass "/Game/Blueprints/Projectiles/Bomb.Bomb_C" (Transformation|GetWorldTransform (Variables|Default|GetArrow1)) "Undefined" 0 0)))
        (:then_1
          (Pawn|Input|AddMovementInput (Variables|Default|GetMovement) 0.5 false))))))

(event EventHitbyPlayer
  (params (Damage :type Float%20%28single-precision%29))
  ;[1 1 1] Getdamage
  (Variables|Default|SetHealthpoints (- (Variables|Default|GetHealthpoints) Damage))
  (if (Variables|Default|GetSoundenabled)
    (Audio|PlaySoundatLocation (Variables|Default|GetGetdamage) "0, 0, 0" "0, 0, 0" 1.0 1.0 0.0 0 0 0))
  (if (< (Variables|Default|GetHealthpoints) 1.0)
    (CallFunction|Death)))

(event EventEntertheCamera
  ;[1 1 1] Behavior
  (Variables|Default|SetMovement "0,-1.200000, 0")
  (Variables|Default|SetIncamera true))

(fn ConstructionScript)